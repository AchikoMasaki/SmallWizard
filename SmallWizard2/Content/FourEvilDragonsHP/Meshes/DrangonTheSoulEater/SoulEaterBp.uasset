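; Soul Eater dragon enemy, driven by a behavior tree started on BeginPlay.
; Pawn sensing sets the "Gördümü" (seen) blackboard key for the MainCharacter, while sphere overlap with that character sets the SoulEaterDuruş flag.
; Health lives on the SoulEaterWidget, cached by the Wİdget1 event.
; ReduceHeal subtracts from it and updates the widget, or at exactly zero flags death, destroys the dragon and spawns Gold.
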(event `self.ReceiveBeginPlay`
  (`AIController.RunBehaviorTree` (`AIBlueprintHelperLibrary.GetAIController` self) "/Game/FourEvilDragonsHP/Meshes/DrangonTheSoulEater/YapayZekaTree.YapayZekaTree"))

(event `Wİdget1`
  (bind _assoul_eater_widget (cast `/Game/Widget/SoulEaterWidget` (`WidgetComponent.GetUserWidgetObject` (`self.Widget`))))
  (set `self.As Soul Eater Widget` _assoul_eater_widget))

(event `self.Sphere.OnComponentBeginOverlap`
  (params (OverlappedComponent :type "PrimitiveComponent Object Reference") (OtherActor :type "Actor Object Reference") (OtherComp :type "PrimitiveComponent Object Reference") (OtherBodyIndex :type Integer) (bFromSweep :type Boolean) (SweepResult :type "HitResult Structure (by ref)"))
  (cast `/Game/ThirdPersonBP/Blueprints/MainCharacter` OtherActor)
  (set `self.SoulEaterDuruş` true))

(event `self.PawnSensing.OnSeePawn`
  (params (Pawn :type "Pawn Object Reference"))
  (cast `/Game/ThirdPersonBP/Blueprints/MainCharacter` Pawn)
  (`BlackboardComponent.SetValueAsBool` (`AIBlueprintHelperLibrary.GetBlackboard` (`AIBlueprintHelperLibrary.GetAIController` self)) "Gördümü" true))

(fn `ReduceHeal`
  (params (value :type "Float (double-precision)"))
  (bind _as_soul_eater_widget (`self.As Soul Eater Widget`))
  (bind _output_get (set `/Game/Widget/SoulEaterWidget.SoulEaterHeal` (- (`/Game/Widget/SoulEaterWidget.SoulEaterHeal` _as_soul_eater_widget) value) _as_soul_eater_widget))
  (if (== _output_get 0.0)
    (set `self.SoulÖlüm` true)
    (`self.K2_DestroyActor`)
    (`|SpawnActorFromClass` "/Game/BluePrint/Gold.Gold_C" (`self.GetTransform`) "Undefined" "OverrideRootScale" null null)
    (else
      (`/Game/Widget/SoulEaterWidget.Update` _as_soul_eater_widget _output_get))))

(fn `UserConstructionScript`)