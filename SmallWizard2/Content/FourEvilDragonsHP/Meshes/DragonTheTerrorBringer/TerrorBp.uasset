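; Blueprint for the Terror Bringer dragon, a damageable actor that drops Gold when killed.
; It caches the TerrorWidget from its widget component, which stores its health, and flags TerrorEsasDuruş when MainCharacter enters its sphere.
; ReduceTerrorHeal subtracts damage and refreshes the widget, or at exactly zero health sets the death flag, destroys the actor and spawns Gold at its transform.
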(event `self.ReceiveBeginPlay`
  (bind _asterror_widget (cast `/Game/Widget/TerrorWidget` (`WidgetComponent.GetUserWidgetObject` (`self.Widget`))))
  (set `self.As Terror Widget` _asterror_widget))

(event `self.Sphere.OnComponentBeginOverlap`
  (params (OverlappedComponent :type "PrimitiveComponent Object Reference") (OtherActor :type "Actor Object Reference") (OtherComp :type "PrimitiveComponent Object Reference") (OtherBodyIndex :type Integer) (bFromSweep :type Boolean) (SweepResult :type "HitResult Structure (by ref)"))
  (cast `/Game/ThirdPersonBP/Blueprints/MainCharacter` OtherActor)
  (set `self.TerrorEsasDuruş` true))

(fn `ReduceTerrorHeal`
  (params (Value :type "Float (double-precision)"))
  (bind _as_terror_widget (`self.As Terror Widget`))
  (bind _output_get (set `/Game/Widget/TerrorWidget.TerrorHeal` (- (`/Game/Widget/TerrorWidget.TerrorHeal` _as_terror_widget) Value) _as_terror_widget))
  (if (== _output_get 0.0)
    (set `self.TerrorÖlüm` true)
    (`self.K2_DestroyActor`)
    (`|SpawnActorFromClass` "/Game/BluePrint/Gold.Gold_C" (`self.GetTransform`) "Undefined" "OverrideRootScale" null null)
    (else
      (`/Game/Widget/TerrorWidget.UpdateTerror` _as_terror_widget _output_get))))

(fn `UserConstructionScript`)