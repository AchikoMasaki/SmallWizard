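; Nightmare dragon enemy actor with a health widget, which drops Gold when killed.
; A MainCharacter entering its Sphere sets the NightEsasDuruş (main stance) flag.
; NightReduceHeal subtracts damage from the health stored in the widget itself, then refreshes the display.
; At exactly zero health it instead sets NightÖlüm (death), destroys the actor and spawns Gold at its transform.
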(event `self.ReceiveBeginPlay`
  (bind _asnight_widget (cast `/Game/Widget/NightWidget` (`WidgetComponent.GetUserWidgetObject` (`self.Widget`))))
  (set `self.As Night Widget` _asnight_widget))

(event `self.Sphere.OnComponentBeginOverlap`
  (params (OverlappedComponent :type "PrimitiveComponent Object Reference") (OtherActor :type "Actor Object Reference") (OtherComp :type "PrimitiveComponent Object Reference") (OtherBodyIndex :type Integer) (bFromSweep :type Boolean) (SweepResult :type "HitResult Structure (by ref)"))
  (cast `/Game/ThirdPersonBP/Blueprints/MainCharacter` OtherActor)
  (set `self.NightEsasDuruş` true))

(fn `NightReduceHeal`
  (params (Value :type "Float (double-precision)"))
  (bind _as_night_widget (`self.As Night Widget`))
  (bind _output_get (set `/Game/Widget/NightWidget.NightHeal` (- (`/Game/Widget/NightWidget.NightHeal` _as_night_widget) Value) _as_night_widget))
  (if (== _output_get 0.0)
    (set `self.NightÖlüm` true)
    (`self.K2_DestroyActor`)
    (`|SpawnActorFromClass` "/Game/BluePrint/Gold.Gold_C" (`self.GetTransform`) "Undefined" "OverrideRootScale" null null)
    (else
      (`/Game/Widget/NightWidget.NightUpdate` _as_night_widget _output_get))))

(fn `UserConstructionScript`)